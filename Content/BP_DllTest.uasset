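; Test Blueprint that checks runtime loading of the RapidLib plugin DLL and a string call into it.
; On BeginPlay it imports the DLL, binds its char-array method, passes in a test string and prints the returned result.
; A failed DLL or method import prints an error instead.
; Tick calls FreeDLL every frame, with no check on whether the library is loaded.
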(event `self.ReceiveBeginPlay`
  (bind _returnvalue (`CreateAndLinkDLLTutBFL.importDLL` "Rapidlib" "RapidLibPlugin.dll"))
  (if _returnvalue
    (`|ExecutionSequence`
      (:`then_0`
        (bind _returnvalue_2 (`CreateAndLinkDLLTutBFL.importMethodGetCharArray`))
        (if _returnvalue_2
          (bind _returnvalue_3 (`CreateAndLinkDLLTutBFL.getCharArrayFromDll` "BLA BLA BLA THIS IS A "))
          (`KismetSystemLibrary.PrintString` _returnvalue_3)
          (else
            (`KismetSystemLibrary.PrintString` "Error importing getchararray method from dll")))))
    (else
      (`KismetSystemLibrary.PrintString` "ERROR LOADING DLL SHIT "))))

(event `self.ReceiveTick`
  (params (DeltaSeconds :type "Float (single-precision)"))
  (`CreateAndLinkDLLTutBFL.freeDLL`))

(fn `UserConstructionScript`)